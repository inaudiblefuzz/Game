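; Base gun Blueprint for the first-person character, snapping its mesh to the arms' GripPoint and managing ammo and firing.
; Start and stop events only set IsFiring; nothing here calls FireBullet.
; FireBullet either camera-traces and pushes physics objects, or spawns GunClass at the barrel, decrementing ammo a second time.
; AddAmmo caps refills at the maximum, and GetAmmoClass exposes the ammo type.
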(event Custom|StartShooting
  (Variables|Default|SetIsFiring true))

(event Custom|StopShooting
  (Variables|Default|SetIsFiring false))

(event EventAddPrimaryAmmo
  (params (Rockets :type Integer) (Rails :type Integer) (AmmoCount :type Integer))
  (CallFunction|AddAmmo AmmoCount))

(fn ConstructionScript
  (Transformation|AttachComponentToComponent (Variables|Default|GetGuns) (Variables|Default|GetArms) "GripPoint" "SnapToTarget" "SnapToTarget" "SnapToTarget" true))

(fn FireBullet
  ;[1 1 1] Line trace
  (Audio|PlaySoundatLocation "/Game/StarterContent/Audio/Explosion01.Explosion01" "0, 0, 0" "0, 0, 0" 1.0 1.0 0.0 0 0 0)
  (if (> (Variables|Default|GetAmmoCurrent) 0)
    (Math|Integer|DecrementInt (Variables|Default|GetAmmoCurrent) ; Enables Ammo Count (Subtract)
      (:%20%20
        (if (Variables|Default|GetIsHitScan)
          (bind _asfirst_person_character (Utilities|Casting|CastToFirstPersonCharacter (Actor|GetParentActor)))
          (if true
            (LocalVariables|SetGunDirection (Math|Vector|GetForwardVector (Transformation|GetWorldRotation (Variables|/Game/Player/Blueprints/FirstPersonCharacter.FirstPersonCharacter_C|GetFirstPersonCamera _asfirst_person_character))))
            (bind _outhit (Collision|LineTraceByChannel (Transformation|GetWorldLocation (Variables|/Game/Player/Blueprints/FirstPersonCharacter.FirstPersonCharacter_C|GetFirstPersonCamera _asfirst_person_character)) (+ (Transformation|GetWorldLocation (Variables|/Game/Player/Blueprints/FirstPersonCharacter.FirstPersonCharacter_C|GetFirstPersonCamera _asfirst_person_character)) (* (Math|Vector|GetForwardVector (Transformation|GetWorldRotation (Variables|/Game/Player/Blueprints/FirstPersonCharacter.FirstPersonCharacter_C|GetFirstPersonCamera _asfirst_person_character))) 2e+03)) "TraceTypeQuery1" false 0 "ForDuration"))
            (if (.bBlockingHit (Collision|BreakHitResult _outhit)) ; Did we hit something?
              (if (Physics|IsSimulatingPhysics (.HitComponent (Collision|BreakHitResult _outhit)) "None")
                (Physics|AddImpulseatLocation (.HitComponent (Collision|BreakHitResult _outhit)) (* (LocalVariables|GetGunDirection) 5e+06) (.ImpactPoint (Collision|BreakHitResult _outhit)) "None") ; Applying physics to hit
                (Animation|Montage|MontagePlay (Components|SkeletalMesh|GetAnimInstance (Variables|Default|GetArms)) "/Game/Animations/DefaultAnimations/FirstPersonFire_Montage.FirstPersonFire_Montage" 1.0 "MontageLength" 0.0 true) ; Firing animation
              )))
          (else
            ;[1 1 1] Default firing
            (bind _asfirst_person_character_2 (Utilities|Casting|CastToFirstPersonCharacter (Actor|GetParentActor)))
            (if (> (Variables|Default|GetAmmoCurrent) 0)
              (Game|SpawnActorfromClass (Variables|Default|GetGunClass) (Math|Transform|MakeTransform (Transformation|GetWorldLocation (Variables|Default|GetBarrelReference)) (Transformation|GetWorldRotation (Variables|/Game/Player/Blueprints/FirstPersonCharacter.FirstPersonCharacter_C|GetFirstPersonCamera _asfirst_person_character_2)) "1,1,1") "Undefined" 0 0) ; Spawn the gun
              ;;[0 0.4488 1] Firing Animation
              (Animation|Montage|MontagePlay (Components|SkeletalMesh|GetAnimInstance (Variables|Default|GetArms)) "/Game/Animations/DefaultAnimations/FirstPersonFire_Montage.FirstPersonFire_Montage" 1.0 "MontageLength" 0.0 true) ; Firing animation
              (Audio|PlaySoundatLocation (Variables|Default|GetGunAudio) "0, 0, 0" "0, 0, 0" 1.0 1.0 0.0 0 0 0)
              (Math|Integer|DecrementInt (Variables|Default|GetAmmoCurrent)) ; Enables Ammo Count (Subtract)
            )))))))

(fn AddAmmo
  (params (InputPin :type Integer))
  ;[1 1 1] Do we have space for more ammo?
  (if (< (Variables|Default|GetAmmoCurrent) (Variables|Default|GetAmmoMax))
    ;[1 1 1] Is the difference between our currentAmmo count and max less or equal to how much we want to add?
    (if (<= (- (Variables|Default|GetAmmoMax) (Variables|Default|GetAmmoCurrent)) InputPin)
      ;[1 1 1] Just top the current up to max
      (Variables|Default|SetAmmoCurrent (Variables|Default|GetAmmoMax))
      (else
        ;[1 1 1] Add the ammo to current we still need more.
        (Variables|Default|SetAmmoCurrent (+ (Variables|Default|GetAmmoCurrent) InputPin))))
    (else
      (Development|PrintString "Ammo Full!"))))

(fn GetAmmoClass
  (if (Utilities|IsValidClass (Variables|Default|GetAmmoClass))
    (return (Variables|Default|GetAmmoClass))))