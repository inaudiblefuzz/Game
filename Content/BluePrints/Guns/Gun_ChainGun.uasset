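; Chain gun weapon Blueprint that provides automatic fire on top of a parent gun class.
; StartShooting calls the parent, fires one bullet immediately, then sets a looping timer that calls FireBullet at the FireRate interval.
; StopShooting calls the parent and clears and invalidates the stored timer handle to end the fire loop.
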(event EventStartShooting
  (|CallParentFunction)
  (CallFunction|FireBullet) ; Instant Fire Bullet
  (bind _returnvalue (Utilities|Time|SetTimerbyFunctionName 0 "FireBullet" (Variables|Default|GetFireRate) true))
  (Variables|Default|SetGunTimer _returnvalue))

(event EventStopShooting
  (|CallParentFunction)
  (Utilities|Time|ClearandInvalidateTimerbyHandle (Variables|Default|GetGunTimer)))

(fn ConstructionScript
  (|CallParentFunction))