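; Parent Blueprint for ammo pickups that top up the player's equipped gun and respawn.
; On trigger overlap, it compares the gun's ammo class with its own and sends the amount via Blueprint Interface messages, printing a warning on mismatch.
; A DoOnce gates hiding the actor until a Timeline finishes.
; Ammo is granted before that gate and the trigger stays active, so hidden pickups still give ammo.
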(event OnComponentBeginOverlap(Trigger)
  (params (OverlappedComponent :type Primitive%20Component%20Object%20Reference) (OtherActor :type Actor%20Object%20Reference) (OtherComp :type Primitive%20Component%20Object%20Reference) (OtherBodyIndex :type Integer) (bFromSweep :type Boolean) (SweepResult :type Hit%20Result%20Structure%20%28by%20ref%29))
  ;[1 1 1] Make sure the character ran over the pickup
  (bind _asfirst_person_character (Utilities|Casting|CastToFirstPersonCharacter OtherActor))
  ;[1 1 1] Get the equipped gun and make sure its valid
  (bind _gun (Class|BPICharacter|GetEquippedGun(Message) _asfirst_person_character))
  (Utilities|IsValid _gun
    (:Is%20Valid
      ;[1 1 1] Check that the Ammo used by the gun is the same as this pickup
      (bind _ammoused (Class|BPIGuns|GetAmmoClass(Message) _gun))
      (if (== _ammoused (Variables|Default|GetAmmoClass))
        ;[1 1 1] Add the Ammo to our Gun by sending a message through the BPI added to the Gun_Parent class
        (Class|BPIGuns|AddPrimaryAmmo(Message) _gun 0 0 (Variables|Default|GetAmmoAmount))
        ;[1 1 1] Use our DoOnce Gate so we can controll the respawn timer (Timeline)
        (Utilities|FlowControl|DoOnce false :!label _label
          (:Completed
            ;[1 1 1] Hide the Pickup
            (Rendering|SetActorHiddenInGame true)
            ;[1 1 1] Timeline set to 5 secs atm
            (Timeline|RespawnAmmoPickup PlayFromStart
              (:Finished
                ;[1 1 1] UnHide the Pickup then reset the DoOnce Gate
                (Rendering|SetActorHiddenInGame false)
                (goto _label Reset)))))
        (else
          (Development|PrintString "Wrong Ammo!"))))))

(event Collision|EventActorBeginOverlap
  (params (OtherActor :type Actor%20Object%20Reference)))

(event EventTick
  (params (DeltaSeconds :type Float%20%28single-precision%29)))

(fn ConstructionScript)